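; Player character Blueprint with a grappling hook, which creates the HUD on BeginPlay.
; A looping timer shows the hook mesh while grappling, rotating it along the line to the grapple point, and hides it otherwise.
; Tick eases control rotation roll back to zero while Orient is set.
; A helper toggles pawn-controlled camera rotation and look input, and a debug key emits a noise event.
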(event Custom|ResetOrientation
  (params (DeltaTime :type Float%20%28double-precision%29))
  (bind _returnvalue (Game|GetPlayerController 0))
  (bind _returnvalue_2 (Pawn|GetControlRotation _returnvalue :!class /Script/Engine.Controller))
  ;[0.15 0.15 0.15 0.5] Reset Orientation
  (Pawn|SetControlRotation (Game|GetPlayerController 0) (Math|Interpolation|RInterpTo (Pawn|GetControlRotation _returnvalue :!class /Script/Engine.Controller) (Math|Rotator|MakeRotator 0.0 (.pitch _returnvalue_2) (.yaw _returnvalue_2)) DeltaTime (* DeltaTime 3e+02)))
  (if (Math|Float|NearlyEqual(Float) (.roll _returnvalue_2) 0.0 0.01)
    (Variables|Default|SetbOrient false)))

(event Custom|HookFollowEvent
  (bind _returnvalue (Class|VSlicesCharacter|GetGrapplingHookComponent))
  ;[0.15 0.15 0.15 0.5] Hook follow visuals
  (Utilities|IsValid _returnvalue
    (:Is%20Valid
      (if (Class|GrapplingHookComponent|IsGrappling _returnvalue)
        (Variables|Default|GetCable
          (:then
            (bind _sm_grapplinghook (Variables|Default|GetSM_GrapplingHook)
              (:then
                (if (Rendering|IsVisible _sm_grapplinghook)
                  _
                  (else
                    (Rendering|SetVisibility _sm_grapplinghook true false)))
                (Transformation|SetWorldRotation _sm_grapplinghook (Math|Rotator|MakeRotator (.roll (Math|Rotator|FindLookatRotation (Class|GrapplingHookComponent|GetGrappleLocation _returnvalue) (Transformation|GetWorldLocation _sm_grapplinghook))) (+ (.pitch (Math|Rotator|FindLookatRotation (Class|GrapplingHookComponent|GetGrappleLocation _returnvalue) (Transformation|GetWorldLocation _sm_grapplinghook))) 9e+01) (.yaw (Math|Rotator|FindLookatRotation (Class|GrapplingHookComponent|GetGrappleLocation _returnvalue) (Transformation|GetWorldLocation _sm_grapplinghook)))) false false))
              (:else)))
          (:else
            (Utilities|Time|ClearandInvalidateTimerbyHandle (Variables|Default|GetHookFollowTimerHandle))))
        (else
          (bind _sm_grapplinghook_2 (Variables|Default|GetSM_GrapplingHook)
            (:then
              (Rendering|SetVisibility _sm_grapplinghook_2 false false))
            (:else)))))
    (:Is%20Not%20Valid
      (Class|VSlicesCharacter|WarnMissingComponent (Utilities|GetClass _returnvalue)))))

(event EventBeginPlay
  ;[0.15 0.15 0.15 0.5] Setup
  (bind _returnvalue (UserInterface|CreateWidget "/Game/UI/WBP_HUD.WBP_HUD_C"))
  (bind _output_get (Variables|Default|SetHUD _returnvalue))
  (UserInterface|Viewport|AddtoViewport _output_get 0)
  (bind _returnvalue_2 (Utilities|Time|SetTimerbyEvent (EventDispatchers|CreateEvent :!event Custom|HookFollowEvent) 0.1 true))
  (Variables|Default|SetHookFollowTimerHandle _returnvalue_2))

(event EventTick
  (params (DeltaSeconds :type Float%20%28single-precision%29))
  ;[0.15 0.15 0.15 0.5] Tick
  (Variables|Default|GetbOrient
    (:then
      (CallFunction|ResetOrientation DeltaSeconds))
    (:else)))

(event Input|KeyboardEvents|DebugKeyC
  (params (Key :type Key%20Structure :default "None") (ActionValue :type Input%20Action%20Value%20Structure))
  (:Pressed
    (Class|AISenseHearing|ReportNoiseEvent (Transformation|GetActorLocation) 1e+02 self 0.0 "None")
    (Development|PrintString "Made a noise" true true "(R=1.000000,G=0.658686,B=0.274690,A=1.000000)")))

(fn ConstructionScript)

(fn SetCameraRotation
  (params (Use%20Pawn%20Control%20Rotation :type Boolean))
  (bind _output_get (Variables|/Script/Engine.CameraComponent|SetbUsePawnControlRotation (Variables|Default|GetFollowCamera) Use%20Pawn%20Control%20Rotation))
  (Input|SetIgnoreLookInput (Game|GetPlayerController 0) (not _output_get)))