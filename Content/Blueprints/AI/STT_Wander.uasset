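; A StateTree task that makes an AI pawn wander around its current location.
; On entering the state, it moves the pawn to a random reachable navmesh point within a radius.
; After arriving, it waits on a timer before finishing successfully, while a failed move finishes the task as failed.
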(event Custom|EndWait
  (StateTree|FinishTask true))

(event EventLatentEnterState
  (params (Transition :type State%20Tree%20Transition%20Result%20Structure%20%28by%20ref%29))
  (bind _pawn (Variables|Default|GetPawn))
  (AI|AIMoveTo _pawn (.RandomLocation (AI|Navigation|GetRandomReachablePointinRadius (Transformation|GetActorLocation _pawn) (Variables|Default|GetRadius) 0 0)) 0 5.0 false
    (:OnSuccess
      (Utilities|Time|SetTimerbyEvent (EventDispatchers|CreateEvent :!event Custom|EndWait) (Variables|Default|GetWaitTime)))
    (:OnFail
      (StateTree|FinishTask false))))