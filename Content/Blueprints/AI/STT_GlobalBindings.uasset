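; StateTree task that feeds AI perception of the player character into the StateTree, likely as a global task.
; On entering state, it binds to the AI controller's perception update and ignores any actor other than player 0.
; It writes the player to the target actor property reference when sensed, or clears it otherwise.
; It then sends an AI.SensedActor event carrying the stimulus as an instanced struct payload.
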(event EventLatentEnterState
  (params (Transition :type State%20Tree%20Transition%20Result%20Structure%20%28by%20ref%29))
  (CallFunction|CreateBindings))

(fn CreateBindings
  (EventDispatchers|BindEventtoOnTargetPerceptionUpdated (Variables|/Game/Blueprints/AI/AIC_NPC.AIC_NPC_C|GetAIPerception (Variables|Default|GetAIController)) (EventDispatchers|CreateEvent :!event BindingPerceptionUpdate)))

(fn BindingPerceptionUpdate
  (params (Actor :type Actor%20Object%20Reference) (Stimulus :type AI%20Stimulus%20Structure))
  (if (== Actor (Game|GetPlayerCharacter 0))
    (bind _reference (|StateTreeBlueprintPropertyRef (Variables|Default|GetTargetActorPropRef))
      (:Succeeded
        (|SetBy-RefVar _reference (select (.bSuccessfullySensed (Utilities|Struct|BreakAIStimulus Stimulus)) Actor 0))
        (bind _returnvalue (Utilities|InstancedStruct|MakeInstancedStruct Stimulus))
        (Class|StateTreeNodeBlueprintBase|SendEvent (Utilities|Struct|MakeStateTreeEvent "(TagName=\"AI.SensedActor\")" _returnvalue))))))