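; AI controller for NPCs that patrol a spline path, chase a seen player and investigate noises.
; On possess it gets the patrol path from the pawn, then the Patrol event walks its spline points in a loop.
; Perception updates send Chase, Patrol or Investigate events to the StateTree based on sight and hearing.
; Heard stimuli also trigger a move to their location, signalling investigation finish on arrival or returning to Patrol on failure.
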(event OnPerceptionUpdated(AIPerception)
  (params (UpdatedActors :type Array%20of%20Actor%20Object%20References))
  (bind _statetreeai (Variables|Default|GetStateTreeAI))
  (bind _statetreeai_2 (Variables|Default|GetStateTreeAI))
  ;[0.15 0.15 0.15 0.5] Perception Update
  (for _array_element UpdatedActors
    (Utilities|FlowControl|Sequence
      (:then_0
        (bind (_array_element_2 _successfully_sensed _sensedactor) (CallFunction|CanSenseActor _array_element "NewEnumerator0"))
        (if _successfully_sensed
          (Variables|Default|SetPlayer _sensedactor)
          (Gameplay|StateTree|SendStateTreeEvent _statetreeai_2 (Utilities|Struct|MakeStateTreeEvent "(TagName=\"Chase\")") :!class /Script/GameplayStateTreeModule.StateTreeComponent)
          (else
            (Variables|Default|SetPlayer 0)
            (Gameplay|StateTree|SendStateTreeEvent _statetreeai_2 (Utilities|Struct|MakeStateTreeEvent "(TagName=\"Patrol\")") :!class /Script/GameplayStateTreeModule.StateTreeComponent))))
      (:then_1
        (bind (_array_element_3 _successfully_sensed_2) (CallFunction|CanSenseActor _array_element "NewEnumerator1"))
        (if _successfully_sensed_2
          (AI|AIMoveTo (Variables|Default|GetNPC) (.StimulusLocation (Utilities|Struct|BreakAIStimulus _array_element_3)) 0 5.0 false
            (:then
              (Gameplay|StateTree|SendStateTreeEvent _statetreeai (Utilities|Struct|MakeStateTreeEvent "(TagName=\"Investigate\")") :!class /Script/GameplayStateTreeModule.StateTreeComponent))
            (:OnSuccess
              (Default|CallOnInvestigateFinish))
            (:OnFail
              (Gameplay|StateTree|SendStateTreeEvent _statetreeai (Utilities|Struct|MakeStateTreeEvent "(TagName=\"Patrol\")") :!class /Script/GameplayStateTreeModule.StateTreeComponent))))))))

(event Custom|IncreasePatrolPoint
  ;[0.15 0.15 0.15 0.5] Patrol
  (bind _result (Math|Integer|IncrementInt (Variables|Default|GetCurrentPatrolPoint))
    (:%20%20
      (if (> _result (Variables|Default|GetPatrolPointsCount))
        (Variables|Default|SetCurrentPatrolPoint 0))
      (CallFunction|Patrol))))

(event EventPossess
  (params (PossessedPawn :type Pawn%20Object%20Reference))
  ;[0.15 0.15 0.15 0.5] Setup
  (bind _output_get (Variables|Default|SetNPC (.AsCharacter (Utilities|Casting|CastToCharacter PossessedPawn))))
  (bind _patrolpath (Class|BINPC|GetPatrolPath(Message) _output_get))
  (bind _output_get_2 (Variables|Default|SetPatrol%20Path _patrolpath))
  (Variables|Default|SetPatrolPointsCount (Spline|GetNumberOfSplinePoints (Variables|/Game/Blueprints/AI/BP_PatrolPath.BP_PatrolPath_C|GetSpline _output_get_2)))
  (Variables|Default|SetCurrentPatrolPoint 0))

(event EventPatrol
  (bind _npc (Variables|Default|GetNPC))
  ;[0.15 0.15 0.15 0.5] Patrol
  (Variables|/Script/Engine.CharacterMovementComponent|SetMaxWalkSpeed (Variables|/Script/Engine.Character|GetCharacterMovement _npc) (Variables|Default|GetPatrolSpeed))
  (AI|AIMoveTo _npc (Spline|GetLocationatSplinePoint (Variables|/Game/Blueprints/AI/BP_PatrolPath.BP_PatrolPath_C|GetSpline (Variables|Default|GetPatrol%20Path)) (Variables|Default|GetCurrentPatrolPoint) "World") 0 5.0 false
    (:OnSuccess
      (CallFunction|IncreasePatrolPoint))))

(event EventChasePlayer
  ;[0.15 0.15 0.15 0.5] Chase Player
  (bind _player (Variables|Default|GetPlayer)
    (:then
      (AI|AIMoveTo (Variables|Default|GetNPC) "0, 0, 0" _player 5.0 false
        (:then
          (Variables|/Script/Engine.CharacterMovementComponent|SetMaxWalkSpeed (Variables|/Script/Engine.Character|GetCharacterMovement (Variables|Default|GetNPC)) (Variables|Default|GetChaseSpeed)))))
    (:else)))

(fn ConstructionScript)

(fn CanSenseActor
  (params (Actor :type Actor%20Object%20Reference) (Sense :type E_NPC_Senses%20Enum :default "NewEnumerator0"))
  (bind _info (Class|AIPerceptionComponent|GetActorsPerception (Variables|Default|GetAIPerception) Actor))
  (for _array_element (.LastSensedStimuli (Utilities|Struct|BreakActorPerceptionBlueprintInfo _info))
    (bind _returnvalue (Class|AIPerceptionSystem|GetSenseClassforStimulus _array_element))
    (if (== _returnvalue (Utilities|Select :Index Sense :NewEnumerator0 "/Script/AIModule.AISense_Sight" :NewEnumerator1 "/Script/AIModule.AISense_Hearing"))
      (return _array_element (.bSuccessfullySensed (Utilities|Struct|BreakAIStimulus _array_element)) Actor))))